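; BP_Human is a character with a melee attack and one-hit death, driven by a State enum.
; At attack start, the authority sphere-traces forward for pawns and damages other humans; attack end returns Attack to Unarmed.
; Damage while Unarmed triggers death, which resets State to Unarmed, disables movement and capsule collision, and ragdolls the mesh.
; The GameMode and player-killer check after death has no effect.
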(event Custom|CallAttackEnd
  (switch Utilities|FlowControl|Switch|SwitchonEPlayerState (Variables|Default|GetState)
    (:NewEnumerator1
      (Variables|Default|SetState "NewEnumerator0"))))

(event Custom|CallAttackStart
  (bind _returnvalue (Transformation|GetActorLocation))
  (Networking|SwitchHasAuthority
    (:Authority
      (bind _outhits (Collision|MultiSphereTraceForObjects _returnvalue (+ _returnvalue (* (Transformation|GetActorForwardVector) (Variables|Default|GetAttack%20Range))) 15.0 (Utilities|Array|MakeArray "ObjectTypeQuery3") false 0 "None"))
      (for _array_element _outhits
        (bind _asbp_human (Utilities|Casting|CastToBP_Human (.HitActor (Collision|BreakHitResult _array_element))))
        (Utilities|IsValid _asbp_human
          (:Is%20Valid
            (Game|Damage|ApplyDamage _asbp_human 1.0 0 self)))))))

(event Custom|SM_Death
  (bind _mesh (Variables|Character|GetMesh))
  (Utilities|FlowControl|Sequence
    (:then_0
      (Variables|Default|SetState "NewEnumerator0"))
    (:then_1
      (Pawn|Components|CharacterMovement|DisableMovement (Variables|Character|GetCharacterMovement)))
    (:then_2
      (Collision|SetCollisionEnabled (Variables|Collision|GetCapsuleComponent) "NoCollision"))
    (:then_3
      (Collision|SetCollisionEnabled _mesh "PhysicsOnly")
      (Physics|SetSimulatePhysics _mesh true))))

(event Game|Damage|EventAnyDamage
  (params (Damage :type Float%20%28single-precision%29) (DamageType :type Damage%20Type%20Object%20Reference) (InstigatedBy :type Controller%20Object%20Reference) (DamageCauser :type Actor%20Object%20Reference))
  (switch Utilities|FlowControl|Switch|SwitchonEPlayerState (Variables|Default|GetState)
    (:NewEnumerator0
      (Variables|Default|SetState "NewEnumerator2")
      (Utilities|FlowControl|Sequence
        (:then_0
          (CallFunction|SMDeath))
        (:then_1
          (bind _asbp_game_mode (Utilities|Casting|CastToBP_GameMode (Game|GetGameMode)))
          (Utilities|IsValid _asbp_game_mode
            (:Is%20Valid
              (bind _asbp_player (Utilities|Casting|CastToBP_Player DamageCauser))
              (Utilities|IsValid _asbp_player))))))))

(fn ConstructionScript)