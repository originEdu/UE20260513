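; Player character Blueprint that handles attack and sprint actions.
; Each input event calls a CS_ event that forwards to an SM_ event, a naming pattern that suggests server RPC to multicast replication.
; Attack proceeds only from the Unarmed state, checked at both input and CS stages, then sets the Attack state and plays a montage.
; Sprint converts the input into sprint or walk speed and applies it to CharacterMovement.
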(event EventBeginPlay
  (|CallParentFunction) ; This node is disabled and will not be called.\nDrag off pins to build functionality.
)

(event Collision|EventActorBeginOverlap
  (params (OtherActor :type Actor%20Object%20Reference))
  (|CallParentFunction OtherActor) ; This node is disabled and will not be called.\nDrag off pins to build functionality.
)

(event EventTick
  (params (DeltaSeconds :type Float%20%28single-precision%29))
  (|CallParentFunction DeltaSeconds) ; This node is disabled and will not be called.\nDrag off pins to build functionality.
)

(event Custom|CS_Attack
  (switch Utilities|FlowControl|Switch|SwitchonEPlayerState (Variables|Default|GetState)
    (:NewEnumerator0
      (CallFunction|SMAttack))))

(event Custom|CallAttackInput
  (switch Utilities|FlowControl|Switch|SwitchonEPlayerState (Variables|Default|GetState)
    (:NewEnumerator0
      (CallFunction|CSAttack))))

(event Custom|SM_Attack
  (Variables|Default|SetState "NewEnumerator1")
  (Animation|Montage|PlayMontage (Variables|Character|GetMesh) "/Game/Animations/AM_Human.AM_Human" 1.0 0.0 "Default"))

(event Custom|CallSprintInput
  (params (Input :type Boolean))
  (CallFunction|CSSprint Input))

(event Custom|SM_Sprint
  (params (InSpeed :type Float%20%28double-precision%29))
  (Variables|/Script/Engine.CharacterMovementComponent|SetMaxWalkSpeed (Variables|Character|GetCharacterMovement) InSpeed))

(event Custom|CS_Sprint
  (params (Input :type Boolean))
  (CallFunction|SMSprint (select Input (Variables|Default|GetSprintSpeed) (Variables|Default|GetWalkSpeed))))

(fn ConstructionScript
  (|CallParentFunction))