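; Player controller that turns Enhanced Input into actions on the possessed BP_Player and relays kill notifications to the HUD.
; On BeginPlay it caches the pawn and adds the IMC_Player mapping context.
; Movement follows control yaw, look drives controller rotation, and jump, crouch, attack and sprint are forwarded to the pawn.
; SM_ShowKilledUI passes attacker and victim names to BP_HUD only on the local controller.
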(event Input|EnhancedActionEvents|EnhancedInputActionIA_Crouch
  (params (ActionValue :type Boolean) (ElapsedSeconds :type Float%20%28double-precision%29) (TriggeredSeconds :type Float%20%28double-precision%29) (InputAction :type Input%20Action%20Object%20Reference :default "/Game/Inputs/Action/IA_Crouch.IA_Crouch"))
  (bind _playerref (Variables|Default|GetPlayerRef))
  (:Started
    (Character|Crouch _playerref))
  (:Completed
    (Character|UnCrouch _playerref)))

(event Input|EnhancedActionEvents|EnhancedInputActionIA_Move
  (params (ActionValue :type Vector%202D%20Structure) (ElapsedSeconds :type Float%20%28double-precision%29) (TriggeredSeconds :type Float%20%28double-precision%29) (InputAction :type Input%20Action%20Object%20Reference :default "/Game/Inputs/Action/IA_Move.IA_Move"))
  (bind _returnvalue (Pawn|GetControlRotation :!class /Script/Engine.Controller))
  (bind _returnvalue_2 (Pawn|GetControlRotation :!class /Script/Engine.Controller))
  (Pawn|Input|AddMovementInput (Variables|Default|GetPlayerRef) (Math|Vector|GetRightVector (Math|Rotator|MakeRotator (.roll _returnvalue) 0.0 (.yaw _returnvalue))) (.x ActionValue) false)
  (Pawn|Input|AddMovementInput (Variables|Default|GetPlayerRef) (Math|Vector|GetForwardVector (Math|Rotator|MakeRotator (.roll _returnvalue_2) 0.0 (.yaw _returnvalue_2))) (.y ActionValue) false))

(event Input|EnhancedActionEvents|EnhancedInputActionIA_Look
  (params (ActionValue :type Vector%202D%20Structure) (ElapsedSeconds :type Float%20%28double-precision%29) (TriggeredSeconds :type Float%20%28double-precision%29) (InputAction :type Input%20Action%20Object%20Reference :default "/Game/Inputs/Action/IA_Look.IA_Look"))
  (Class|PlayerController|AddYawInput (.x ActionValue))
  (Class|PlayerController|AddPitchInput (.y ActionValue)))

(event Input|EnhancedActionEvents|EnhancedInputActionIA_Jump
  (params (ActionValue :type Boolean) (ElapsedSeconds :type Float%20%28double-precision%29) (TriggeredSeconds :type Float%20%28double-precision%29) (InputAction :type Input%20Action%20Object%20Reference :default "/Game/Inputs/Action/IA_Jump.IA_Jump"))
  (bind _playerref (Variables|Default|GetPlayerRef))
  (:Started
    (Character|Jump _playerref))
  (:Canceled
    (Character|StopJumping _playerref)))

(event Input|EnhancedActionEvents|EnhancedInputActionIA_Attack
  (params (ActionValue :type Boolean) (ElapsedSeconds :type Float%20%28double-precision%29) (TriggeredSeconds :type Float%20%28double-precision%29) (InputAction :type Input%20Action%20Object%20Reference :default "/Game/Inputs/Action/IA_Attack.IA_Attack"))
  (:Triggered
    (Default|CallAttackInput (Variables|Default|GetPlayerRef) :!label _label))
  (:Started
    (goto _label)))

(event Input|EnhancedActionEvents|EnhancedInputActionIA_Sprint
  (params (ActionValue :type Boolean) (ElapsedSeconds :type Float%20%28double-precision%29) (TriggeredSeconds :type Float%20%28double-precision%29) (InputAction :type Input%20Action%20Object%20Reference :default "/Game/Inputs/Action/IA_Sprint.IA_Sprint"))
  (:Started
    (Default|CallSprintInput (Variables|Default|GetPlayerRef) ActionValue :!label _label))
  (:Completed
    (goto _label)))

(event EventBeginPlay
  (bind _self self)
  (bind _returnvalue (PlayerController|LocalPlayerSubsystems|GetEnhancedInputLocalPlayerSubsystem _self))
  (bind _asbp_player (Utilities|Casting|CastToBP_Player (Pawn|GetControlledPawn)))
  (Utilities|IsValid _asbp_player
    (:Is%20Valid
      (Variables|Default|SetPlayerRef _asbp_player)
      (Utilities|IsValid _returnvalue
        (:Is%20Valid
          (Input|AddMappingContext _returnvalue "/Game/Inputs/IMC_Player.IMC_Player" 0 "(bIgnoreAllPressedKeysUntilRelease=True,bForceImmediately=False,bNotifyUserSettings=False)"))))))

(event Custom|SM_ShowKilledUI
  (params (InAttackerName :type String) (InVictimName :type String))
  (if (Pawn|IsLocalPlayerController)
    (bind _asbp_hud (Utilities|Casting|CastToBP_HUD (HUD|GetHUD)))
    (Utilities|IsValid _asbp_hud
      (:Is%20Valid
        (Default|CallShowKilledUI _asbp_hud InAttackerName InVictimName)))))

(fn ConstructionScript)