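; Game mode that populates the level with NPCs and traps and announces human deaths to players.
; On BeginPlay it spawns configured counts of BP_NPC and BP_Trap at random reachable navigation points within a radius, always spawning despite collisions.
; OnHumanDeath passes attacker and victim display names to every BP_PlayerController to show the killed UI.
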(event Custom|SpawnNPC
  (params (InNPCSpawnCount :type Integer))
  (bind _radius (Variables|Default|GetRadius))
  (bind (_randomlocation _returnvalue) (AI|Navigation|GetRandomReachablePointinRadius (Math|Vector|MakeVector 0.0 0.0 88.0) _radius 0 0))
  (for _index (range 1 InNPCSpawnCount)
    (if _returnvalue
      (Game|SpawnActorfromClass "/Game/Blueprints/Character/NPC/BP_NPC.BP_NPC_C" (Math|Transform|MakeTransform _randomlocation "0, 0, 0" "1.000000,1.000000,1.000000") "AlwaysSpawn" "MultiplyWithRoot" 0 0))))

(event Custom|OnHumanDeath
  (params (InAttacker :type Actor%20Object%20Reference) (InVictim :type Actor%20Object%20Reference))
  (bind _outactors (Actor|GetAllActorsOfClass "/Game/Blueprints/Character/Player/BP_PlayerController.BP_PlayerController_C"))
  (for _array_element _outactors
    (Default|SMShowKilledUI _array_element (Utilities|GetDisplayName InAttacker) (Utilities|GetDisplayName InVictim))))

(event Custom|SpawnTraps
  (params (InCnt :type Integer))
  (bind _radius (Variables|Default|GetRadius))
  (bind (_randomlocation _returnvalue) (AI|Navigation|GetRandomReachablePointinRadius (Math|Vector|MakeVector 0.0 0.0 9e+01) _radius 0 0))
  (for _index (range 1 InCnt)
    (if _returnvalue
      (Game|SpawnActorfromClass "/Game/Blueprints/Trap/BP_Trap.BP_Trap_C" (Math|Transform|MakeTransform _randomlocation "0, 0, 0" "1.000000,1.000000,1.000000") "AlwaysSpawn" "MultiplyWithRoot" 0 0))))

(event EventBeginPlay
  (CallFunction|SpawnNPC (Variables|Default|GetNPCSpawnCount))
  (CallFunction|SpawnTraps (Variables|Default|GetTrapSpawnCount)))

(fn ConstructionScript)